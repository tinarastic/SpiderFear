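; Game mode for the spider game that handles level progression, game over and quitting.
; On BeginPlay it finds the current level in the GameLevels list and stores the following entry as NextLevel.
; CountEnemies opens NextLevel once no actors tagged "enemy" remain, while GameOver opens the GameOver level.
; Escape exits the game through a console command.
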(event Custom|GameOver
  ;[1 1 1] Game Over
  (Game|OpenLevel(byName) "GameOver"))

(event Custom|CountEnemies
  ;[1 1 1] How many spiders are left?
  (bind _outactors (Actor|GetAllActorswithTag "enemy"))
  (if (== (Utilities|Array|Length _outactors) 0)
    (Game|OpenLevel(byName) (Utilities|String|StringToName (Variables|Default|GetNextLevel)))))

(event EventBeginPlay
  (bind _gamelevels (Variables|Default|GetGameLevels))
  (bind _returnvalue (Game|GetCurrentLevelName true))
  (Variables|Default|SetNextLevel (Utilities|Array|Get(acopy) _gamelevels (+ (Utilities|Array|FindItem _gamelevels _returnvalue) 1))))

(event EventTick
  (params (DeltaSeconds :type Float%20%28single-precision%29)))

(event Input|KeyboardEvents|Escape
  (params (Key :type Key%20Structure :default "None"))
  (:Pressed
    (Development|ExecuteConsoleCommand "exit" 0)))

(fn ConstructionScript)