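; BP_GiantSpider is a giant spider enemy that handles taking damage, hurt reactions and death.
; Each hit spawns an impulse particle on the mesh, but an IsBeingHurt flag ignores further damage during a reaction.
; Non-lethal hits halt movement for a sped-up hurt montage, then restore walking.
; Lethal hits disable movement, play the death montage, destroy the actor and call CountEnemies on SpiderGameMode.
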(event EventBeginPlay)

(event EventTick
  (params (DeltaSeconds :type Float%20%28single-precision%29)))

(event Game|Damage|EventAnyDamage
  (params (Damage :type Float%20%28single-precision%29) (DamageType :type Damage%20Type%20Object%20Reference) (InstigatedBy :type Controller%20Object%20Reference) (DamageCauser :type Actor%20Object%20Reference))
  ;[1 1 1] Taking a hit
  (Effects|SpawnEmitterAttached "/Game/Blueprints/Effect/P_Impulse.P_Impulse" (Variables|Character|GetMesh) "None" "0, 0, 0" "0, 0, 0" "1.000000,1.000000,1.000000" "KeepRelativeOffset" false)
  (if (not (Variables|Default|GetIs%20Being%20Hurt))
    (Variables|Default|SetIs%20Being%20Hurt true) ; Set this to stop other events firing during a hit
    (bind _output_get (Variables|Default|SetHealth (- (Variables|Default|GetHealth) Damage)))
    (if (<= _output_get 0.0)
      (Pawn|Components|CharacterMovement|DisableMovement (Variables|Character|GetCharacterMovement))
      (bind _returnvalue (Animation|PlayAnimMontage "/Game/Blueprints/Spider/Animation/DeathMontage.DeathMontage" 1.0 "None"))
      (Utilities|FlowControl|Delay _returnvalue)
      (Actor|DestroyActor)
      (bind _asspider_game_mode (Utilities|Casting|CastToSpiderGameMode (Game|GetGameMode)))
      (Default|CountEnemies _asspider_game_mode)
      (else
        (Pawn|Components|CharacterMovement|SetMovementMode (Variables|Character|GetCharacterMovement) "MOVE_None" 0)
        (bind _returnvalue_2 (Animation|PlayAnimMontage "/Game/Blueprints/Spider/Animation/SpiderHurtMontage.SpiderHurtMontage" 3.0 "None"))
        (Utilities|FlowControl|Delay _returnvalue_2)
        (Variables|Default|SetIs%20Being%20Hurt false)
        (Pawn|Components|CharacterMovement|SetMovementMode (Variables|Character|GetCharacterMovement) "MOVE_Walking" 0)))))

(fn ConstructionScript)