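; AI controller base that runs the spider behavior tree and acquires players as enemies.
; On perception updates, while no valid Enemy is set and IsWalkingAway is false, it scans sight-perceived actors for a living MotionControllerPawn.
; The first match is written to the Enemy blackboard key for the behavior tree.
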(event OnPerceptionUpdated(AIPerception)
  (params (UpdatedActors :type Array%20of%20Actor%20Object%20References))
  (bind _returnvalue (AI|GetBlackboard 0))
  (bind _returnvalue_2 (Utilities|Name|MakeLiteralName "Enemy"))
  (Utilities|IsValid (AI|Components|Blackboard|GetValueasObject _returnvalue _returnvalue_2)
    (:Is%20Not%20Valid
      (if (not (Variables|Default|GetIs%20Walking%20Away))
        (bind _array_element (Utilities|Array|ForEachLoopwithBreak (Class|AIPerceptionComponent|GetCurrentlyPerceivedActors (Variables|Default|GetAIPerception) "/Script/AIModule.AISense_Sight") :!label _label)
          (:LoopBody
            (bind _asmotion_controller_pawn (Utilities|Casting|CastToMotionControllerPawn _array_element))
            (if (not (Variables|/Game/Blueprints/VirtualRealityBP/Blueprints/MotionControllerPawn.MotionControllerPawn_C|GetIs%20Dead _asmotion_controller_pawn))
              (AI|Components|Blackboard|SetValueasObject _returnvalue _returnvalue_2 _asmotion_controller_pawn)
              (goto _label Break))))))))

(event EventBeginPlay
  (AI|RunBehaviorTree "/Game/Blueprints/Spider-BT.Spider-BT"))

(fn ConstructionScript)