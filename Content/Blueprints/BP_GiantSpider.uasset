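; BP_GiantSpider is a giant spider character that takes damage, dies and respawns itself.
; On BeginPlay it stores its spawn location and picks a random navigable point nearby as NextSpawnLocation, which is not used afterwards.
; AnyDamage reduces Health; at zero it disables movement and waits out the death montage.
; It then destroys itself and spawns a replacement running SpiderBT at the original spawn location.
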(event EventBeginPlay
  (bind _output_get (Variables|Default|SetMy%20Spawn%20Location (Transformation|GetActorLocation)))
  (bind _randomlocation (Class|NavigationSystemV1|GetRandomLocationinNavigableRadius _output_get 2e+03 0 0))
  (Variables|Default|SetNext%20Spawn%20Location _randomlocation))

(event EventTick
  (params (DeltaSeconds :type Float%20%28single-precision%29)))

(event Game|Damage|EventAnyDamage
  (params (Damage :type Float%20%28single-precision%29) (DamageType :type Damage%20Type%20Object%20Reference) (InstigatedBy :type Controller%20Object%20Reference) (DamageCauser :type Actor%20Object%20Reference))
  (bind _output_get (Variables|Default|SetHealth (- (Variables|Default|GetHealth) Damage)))
  (if (<= _output_get 0.0)
    (Pawn|Components|CharacterMovement|DisableMovement (Variables|Character|GetCharacterMovement))
    (bind _returnvalue (Animation|PlayAnimMontage "/Game/Blueprints/DeathMontage.DeathMontage" 1.0 "None"))
    (Utilities|FlowControl|Delay _returnvalue)
    (Actor|DestroyActor)
    (AI|SpawnAIFromClass "BP_GiantSpider_C" "/Game/Blueprints/Spider-BT.Spider-BT" (Variables|Default|GetMy%20Spawn%20Location) "0, 0, 0" false)))

(fn ConstructionScript)